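; BP_Pacman is the Pac-Man pawn, with an animated mouth and a timed speed power-up.
; Tick feeds a 0.2-second Delay that toggles the visibility of the open and closed components, making the mouth chomp.
; Movement uses FloatingPawnMovement, set to normal speed and acceleration at BeginPlay.
; ApplyPowerUpEffect swaps in power-up values, then an event Delay restores normal movement, without extending on repeat calls mid-effect.
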(event `self.ReceiveBeginPlay`
  (`self.ApplyNormalMovement`))

(event `self.ReceiveTick`
  (params (DeltaSeconds :type "Float (single-precision)"))
  (`KismetSystemLibrary.Delay` 0.2)
  (`self.PlayMouthAnimation`))

(event `PowerUpAppliedEvent`
  (`KismetSystemLibrary.Delay` (`self.PowerUpEffectDuration`))
  (`self.ApplyNormalMovement`))

(fn `ApplyNormalMovement`
  (`|ExecutionSequence`
    (:`then_0`
      (set `FloatingPawnMovement.MaxSpeed` (`self.NormalSpeed`) (`self.FloatingPawnMovement`)))
    (:`then_1`
      (set `FloatingPawnMovement.Acceleration` (`self.NormalAcceleration`) (`self.FloatingPawnMovement`)))))

(fn `ApplyPowerUpEffect`
  (`|ExecutionSequence`
    (:`then_0`
      (set `FloatingPawnMovement.MaxSpeed` (`self.PowerUpSpeed`) (`self.FloatingPawnMovement`)))
    (:`then_1`
      (set `FloatingPawnMovement.Acceleration` (`self.PowerUpAcceleration`) (`self.FloatingPawnMovement`)))
    (:`then_2`
      (`self.PowerUpAppliedEvent`))))

(fn `PlayMouthAnimation`
  (`SceneComponent.ToggleVisibility` (`self.Pacman-Open`) false)
  (`SceneComponent.ToggleVisibility` (`self.Pacman-Closed`) false))

(fn `UserConstructionScript`)