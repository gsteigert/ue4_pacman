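; Pac-Man enemy that chases the player, flees when a power-up is eaten and can itself be eaten while vulnerable.
; Each unfrozen tick, AIMoveTo targets the player, or Origin when Vulnerable or Dead.
; Hunt starts on first tick and on overlapping BP_Enemy_Start; power-up events call Run.
; State changes swap visible meshes and Pawn collision; hits either kill Pacman or the enemy.
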(event `OnFoodieEatenEvent`
  (params (foodieType :type "EFoodieType Enum" :default "Regular"))
  (`self.Run`))

(event `self.ReceiveBeginPlay`
  (`|ExecutionSequence`
    (:`then_0`
      (bind _outactors (`GameplayStatics.GetAllActorsOfClass` "/Game/Pacman/Blueprints/BP_Foodie_PowerUp.BP_Foodie_PowerUp_C"))
      (for _array_element _outactors
        (add `FoodieActor.FoodieEatenEvent` _array_element (delegate `OnFoodieEatenEvent`))))
    (:`then_1`
      (add `self.StateChangedEvent` (delegate `StateChangedEvent_Event_0`)))))

(event `StateChangedEvent_Event_0` :!signature `self.StateChangedEvent`
  (params (newState :type "EEnemyState Enum" :default "Default"))
  (`self.UpdateVisibleMesh`)
  (`self.UpdateCollisionModel`))

(event `self.ReceiveTick`
  (params (DeltaSeconds :type "Float (single-precision)"))
  (`|ExecutionSequence`
    (:`then_0`
      (`/Engine/EditorBlueprintResources/StandardMacros.DoOnce` false
        (:`Completed`
          (`self.Hunt`))))
    (:`then_1`
      (if (not (`self.Frozen`))
        (bind _asaicontroller (cast `AIController` (`self.GetController`)))
        (switch `EEnemyState` (`self.state`)
          (:`Default`
            (`AITask_MoveTo.AIMoveTo` _asaicontroller (0.0 0.0 0.0) (`GameplayStatics.GetPlayerPawn` 0) 0.0 "Disable" "Enable"))
          (:`Vulnerable`
            (`AITask_MoveTo.AIMoveTo` _asaicontroller (0.0 0.0 0.0) (`self.Origin`) 0.0 "Enable" "Enable" :!label _label))
          (:`Dead`
            (goto _label)))))))

(event `self.Sphere.OnComponentHit`
  (params (HitComponent :type "PrimitiveComponent Object Reference") (OtherActor :type "Actor Object Reference") (OtherComp :type "PrimitiveComponent Object Reference") (NormalImpulse :type "Vector Structure") (Hit :type "HitResult Structure (by ref)"))
  (bind _asbp_pacman (cast `/Game/Pacman/Blueprints/BP_Pacman` OtherActor))
  (switch `EEnemyState` (`self.state`)
    (:`Default`
      (`PacmanPawn.Die` _asbp_pacman)
      (`self.Idle`))
    (:`Vulnerable`
      (`self.Die`)
      (`GameplayStatics.PlaySound2D` "/Game/Pacman/Audio/AS_EatEnemyCue.AS_EatEnemyCue" 1.0 1.0 0.0 null null))))

(event `self.Sphere.OnComponentBeginOverlap`
  (params (OverlappedComponent :type "PrimitiveComponent Object Reference") (OtherActor :type "Actor Object Reference") (OtherComp :type "PrimitiveComponent Object Reference") (OtherBodyIndex :type Integer) (bFromSweep :type Boolean) (SweepResult :type "HitResult Structure (by ref)"))
  (cast `/Game/Pacman/Blueprints/BP_Enemy_Start` OtherActor)
  (`self.Hunt`))

(fn `UpdateCollisionModel`
  (bind _sphere (`self.Sphere`))
  (switch `EEnemyState` (`self.state`)
    (:`Default`
      (`PrimitiveComponent.SetCollisionResponseToChannel` _sphere "ECC_Pawn" "ECR_Block" :!label _label))
    (:`Vulnerable`
      (goto _label))
    (:`Dead`
      (`PrimitiveComponent.SetCollisionResponseToChannel` _sphere "ECC_Pawn" "ECR_Ignore" :!label _label_2))
    (:`Idle`
      (goto _label_2))))

(fn `UpdateVisibleMesh`
  (bind _state (`self.state`))
  (`|ExecutionSequence`
    (:`then_0`
      (`SceneComponent.SetVisibility` (`self.Enemy-Default`) (or (`|EnumEquality` "Default" _state) (`|EnumEquality` "Idle" _state)) false))
    (:`then_1`
      (`SceneComponent.SetVisibility` (`self.Enemy-Vulnerable`) (`|EnumEquality` "Vulnerable" _state) false))
    (:`then_2`
      (`SceneComponent.SetVisibility` (`self.Enemy-Dead`) (`|EnumEquality` "Dead" _state) false))))

(fn `UserConstructionScript`)