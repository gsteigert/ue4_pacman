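; BP_Points_Reward is a Pacman score popup actor that shows a point value as moving text and then destroys itself.
; SetRewardValue writes the integer value into the text render component.
; On BeginPlay, a timeline drives both global time dilation for slow motion and the text's interpolated move toward TextTravel.
; The timeline's Update also triggers a one-second Delay before destruction, so that countdown follows dilated time.
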(event `self.ReceiveBeginPlay`
  (bind (_direction _slow_motion _text_location) (`Timeline|Timeline_Travel` :!via `PlayFromStart`)
    (:`Update`
      (`GameplayStatics.SetGlobalTimeDilation` _slow_motion)
      (`SceneComponent.K2_SetRelativeLocation` (`self.TextRender`) (`KismetMathLibrary.VLerp` (0.0 0.0 0.0) (`self.TextTravel`) _text_location) false false)
      (`KismetSystemLibrary.Delay` 1.0)
      (`self.K2_DestroyActor`))))

(fn `SetRewardValue`
  (params (value :type Integer))
  (`TextRenderComponent.K2_SetText` (`self.TextRender`) (`KismetTextLibrary.Conv_IntToText` value)))

(fn `UserConstructionScript`)