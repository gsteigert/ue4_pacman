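; Pacman pawn that manages movement states for normal play, power-ups and death, and animates the character's mouth.
; Power-ups raise FloatingPawnMovement speed and acceleration and activate a trail, then a Delay restores normal movement.
; On the PacmanDied event, max speed drops to zero and a Timeline spins the actor around its yaw.
; A Delay on Tick throttles the chomp, which toggles visibility of open and closed mouth meshes.
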(event `self.ReceiveBeginPlay`
  (`|ExecutionSequence`
    (:`then_0`
      (`self.ApplyNormalMovement`))
    (:`then_1`
      (add `self.PacmanDiedEvent` (delegate `OnPacmanDiedEvent`)))))

(event `OnPacmanDiedEvent`
  (`self.ApplyDeathMovement`)
  (bind (_direction _spin_value) (`Timeline|Spin Timeline` :!via `PlayFromStart`)
    (:`Update`
      (`self.K2_SetActorRelativeRotation` (`KismetMathLibrary.MakeRotator` 0.0 0.0 _spin_value)))))

(event `self.ReceiveTick`
  (params (DeltaSeconds :type "Float (single-precision)"))
  (`KismetSystemLibrary.Delay` 0.2)
  (`self.PlayMouthAnimation`))

(event `PowerUpAppliedEvent`
  (`KismetSystemLibrary.Delay` (`self.PowerUpEffectDuration`))
  (`self.ApplyNormalMovement`))

(fn `ApplyDeathMovement`
  (`|ExecutionSequence`
    (:`then_0`
      (set `FloatingPawnMovement.MaxSpeed` 0.0 (`self.FloatingPawnMovement`)))))

(fn `ApplyNormalMovement`
  (`|ExecutionSequence`
    (:`then_0`
      (set `FloatingPawnMovement.MaxSpeed` (`self.NormalSpeed`) (`self.FloatingPawnMovement`)))
    (:`then_1`
      (set `FloatingPawnMovement.Acceleration` (`self.NormalAcceleration`) (`self.FloatingPawnMovement`)))
    (:`then_2`
      (`ActorComponent.Deactivate` (`self.P_PowerUp_Trail`)))))

(fn `ApplyPowerUpMovement`
  (`|ExecutionSequence`
    (:`then_0`
      (set `FloatingPawnMovement.MaxSpeed` (`self.PowerUpSpeed`) (`self.FloatingPawnMovement`)))
    (:`then_1`
      (set `FloatingPawnMovement.Acceleration` (`self.PowerUpAcceleration`) (`self.FloatingPawnMovement`)))
    (:`then_2`
      (`ActorComponent.Activate` (`self.P_PowerUp_Trail`) false))
    (:`then_3`
      (`self.PowerUpAppliedEvent`))))

(fn `PlayMouthAnimation`
  (`SceneComponent.ToggleVisibility` (`self.SM_Pacman_Open`) false)
  (`SceneComponent.ToggleVisibility` (`self.SM_Pacman_Closed`) false))

(fn `UserConstructionScript`)